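; BP_EchosPlayerCharacter is the player pawn that turns Enhanced Input into four-directional movement.
; On BeginPlay it adds IMC_PlayerInputMapping to the first player controller's input subsystem.
; Separate forward, backward, right and left actions each check that subsystem is valid, then add movement along fixed world axes rather than camera or actor-relative ones, scaled by the action value.
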(event `self.ReceiveBeginPlay`
  (bind _returnvalue (pcsubsystem `EnhancedInputLocalPlayerSubsystem` (`GameplayStatics.GetPlayerController` 0)))
  (`/Engine/EditorBlueprintResources/StandardMacros.IsValid` _returnvalue
    (:`Is Valid`
      (`EnhancedInputSubsystemInterface.AddMappingContext` _returnvalue "/Game/IMC_PlayerInputMapping.IMC_PlayerInputMapping" 0 (struct)))))

(event `self.ReceivePossessed`
  (params (NewController :type "Controller Object Reference")))

(event `EnhancedInput|/Game/IA_MoveFoward`
  (params (ActionValue :type "Float (double-precision)") (ElapsedSeconds :type "Float (double-precision)") (TriggeredSeconds :type "Float (double-precision)") (InputAction :type "InputAction Object Reference" :default "/Game/IA_MoveFoward.IA_MoveFoward"))
  (:`Triggered`
    (`/Engine/EditorBlueprintResources/StandardMacros.IsValid` (pcsubsystem `EnhancedInputLocalPlayerSubsystem` (`GameplayStatics.GetPlayerController` 0)) :!label _label
      (:`Is Valid`
        (`self.AddMovementInput` (-1.0 0.0 0.0) ActionValue))))
  (:`Ongoing`
    (goto _label)))

(event `EnhancedInput|/Game/IA_MoveBackward`
  (params (ActionValue :type "Float (double-precision)") (ElapsedSeconds :type "Float (double-precision)") (TriggeredSeconds :type "Float (double-precision)") (InputAction :type "InputAction Object Reference" :default "/Game/IA_MoveBackward.IA_MoveBackward"))
  (:`Triggered`
    (`/Engine/EditorBlueprintResources/StandardMacros.IsValid` (pcsubsystem `EnhancedInputLocalPlayerSubsystem` (`GameplayStatics.GetPlayerController` 0))
      (:`Is Valid`
        (`self.AddMovementInput` (1.0 0.0 0.0) ActionValue)))))

(event `EnhancedInput|/Game/IA_MoveRight`
  (params (ActionValue :type "Float (double-precision)") (ElapsedSeconds :type "Float (double-precision)") (TriggeredSeconds :type "Float (double-precision)") (InputAction :type "InputAction Object Reference" :default "/Game/IA_MoveRight.IA_MoveRight"))
  (:`Triggered`
    (`/Engine/EditorBlueprintResources/StandardMacros.IsValid` (pcsubsystem `EnhancedInputLocalPlayerSubsystem` (`GameplayStatics.GetPlayerController` 0))
      (:`Is Valid`
        (`self.AddMovementInput` (0.0 -1.0 0.0) ActionValue)))))

(event `EnhancedInput|/Game/IA_MoveLeft`
  (params (ActionValue :type "Float (double-precision)") (ElapsedSeconds :type "Float (double-precision)") (TriggeredSeconds :type "Float (double-precision)") (InputAction :type "InputAction Object Reference" :default "/Game/IA_MoveLeft.IA_MoveLeft"))
  (:`Triggered`
    (`/Engine/EditorBlueprintResources/StandardMacros.IsValid` (pcsubsystem `EnhancedInputLocalPlayerSubsystem` (`GameplayStatics.GetPlayerController` 0))
      (:`Is Valid`
        (`self.AddMovementInput` (0.0 1.0 0.0) ActionValue)))))

(fn `UserConstructionScript`)